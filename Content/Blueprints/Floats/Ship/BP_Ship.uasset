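; BP_Ship is a physics-driven ship that turns and moves according to the state of its BP_Helm child actor, cached on BeginPlay.
; ProcessTurning copies the helm's wheel rotation to WheelTemp and applies yaw torque scaled from that rotation's pitch.
; ProcessRaising pushes the hull along its right vector, scaled by the helm's sail amount.
; ProcessCannons is an empty stub, and nothing in this file calls the Process functions.
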(event `self.ReceiveBeginPlay`
  (bind _asbp_helm (cast `/Game/Blueprints/Floats/Ship/BP_Helm` (`ChildActorComponent.ChildActor` (`self.Helm`))))
  (set `self.HelmReference` _asbp_helm))

(fn `ProcessCannons`)

(fn `ProcessRaising`
  (`PrimitiveComponent.AddForce` (`self.ShipMesh`) (* (`KismetMathLibrary.GetRightVector` (`SceneComponent.K2_GetComponentRotation` (`self.ShipMesh`))) (* (`self.MaxMovementSpeed`) (`/Game/Blueprints/Floats/Ship/BP_Helm.SailAmount` (`self.HelmReference`)))) "None" false))

(fn `ProcessTurning`
  (bind _wheelrotation (`/Game/Blueprints/Floats/Ship/BP_Helm.WheelRotation` (`self.HelmReference`)))
  (`SceneComponent.K2_SetRelativeRotation` (`self.WheelTemp`) _wheelrotation false false)
  (`PrimitiveComponent.AddTorqueInDegrees` (`self.ShipMesh`) (`KismetMathLibrary.MakeVector` 0.0 0.0 (* (.pitch _wheelrotation) (`self.MaxTurningSpeed`))) "None" false))

(fn `UserConstructionScript`)