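; Ship helm, placed as a child actor of BP_Ship, that turns keyboard input into wheel and sail control.
; A/D and W/S set flags for turning the wheel and lowering or raising the sail.
; Each Tick steps wheel pitch within about one turn either way and sail amount between 0 and 1, without delta-time scaling.
; It then calls the parent ship's ProcessTurning and ProcessRaising.
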(event `self.ReceiveBeginPlay`
  (bind _asbp_ship (cast `/Game/Blueprints/Floats/Ship/BP_Ship` (`self.GetParentActor`)))
  (set `self.ShipRef` _asbp_ship))

(event `Key|A`
  (params (Key :type "Key Structure"))
  (:`Pressed`
    (set `self.IsRotatingLeft` true)
    (set `self.IsRotatingRight` false))
  (:`Released`
    (set `self.IsRotatingLeft` false)))

(event `Key|W`
  (params (Key :type "Key Structure"))
  (:`Pressed`
    (set `self.IsRaisingSail` false)
    (set `self.IsLoweringSail` true))
  (:`Released`
    (set `self.IsLoweringSail` false)))

(event `Key|D`
  (params (Key :type "Key Structure"))
  (:`Pressed`
    (set `self.IsRotatingLeft` false)
    (set `self.IsRotatingRight` true))
  (:`Released`
    (set `self.IsRotatingRight` false)))

(event `Key|S`
  (params (Key :type "Key Structure"))
  (:`Pressed`
    (set `self.IsRaisingSail` true)
    (set `self.IsLoweringSail` false))
  (:`Released`
    (set `self.IsRaisingSail` false)))

(event `self.ReceiveTick`
  (params (DeltaSeconds :type "Float (single-precision)"))
  (`self.Turn`)
  (`self.Raise`))

(fn `Raise`
  (if (and (`self.IsRaisingSail`) (> (`self.SailAmount`) 0.0))
    (set `self.SailAmount` (- (`self.SailAmount`) (`self.SailRaiseSpeed`)))
    (elif (and (`self.IsLoweringSail`) (< (`self.SailAmount`) 1.0))
      (set `self.SailAmount` (+ (`self.SailAmount`) (`self.SailDropSpeed`)))))
  (set `self.SailAmount` (`KismetMathLibrary.FClamp` (`self.SailAmount`)))
  (`/Game/Blueprints/Floats/Ship/BP_Ship.ProcessRaising` (`self.ShipRef`)))

(fn `Turn`
  (locals (NewRotation :type "Float (double-precision)"))
  (bind (_wheelrotation_roll _wheelrotation_pitch _wheelrotation_yaw) (`KismetMathLibrary.BreakRotator` (`self.WheelRotation`)))
  (bind (_wheelrotation_roll_2 _wheelrotation_pitch_2) (`KismetMathLibrary.BreakRotator` (`self.WheelRotation`)))
  (bind (_wheelrotation_roll_3 _wheelrotation_pitch_3) (`KismetMathLibrary.BreakRotator` (`self.WheelRotation`)))
  (if (and (`self.IsRotatingLeft`) (> _wheelrotation_pitch_3 -360.0))
    (set `local.NewRotation` (* (`self.WheelTurningSpeed`) -1.0))
    (elif (and (`self.IsRotatingRight`) (< _wheelrotation_pitch_2 360.0))
      (set `local.NewRotation` (`self.WheelTurningSpeed`))
      (else
        (set `local.NewRotation` 0.0))))
  (set `self.WheelRotation` (`KismetMathLibrary.MakeRotator` _wheelrotation_roll (+ _wheelrotation_pitch (`local.NewRotation`)) _wheelrotation_yaw))
  (`/Game/Blueprints/Floats/Ship/BP_Ship.ProcessTurning` (`self.ShipRef`)))

(fn `UserConstructionScript`)